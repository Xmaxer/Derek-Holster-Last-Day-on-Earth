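; Moveable object Blueprint that shows a floating name and weight label when the player aims the gravity tool at it.
; On Tick, each instance line-traces from Derek's CastingPoint using the tool's grab distance and object types, then updates the hit Moveable_BP's hover widget.
; The label sits atop the object's bounds, faces the CastingPoint and shrinks for longer text.
; It hides while the tool is holding or the trace finds no moveable.
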(event EventBeginPlay)

(event Collision|EventActorBeginOverlap
  (params (OtherActor :type Actor%20Object%20Reference)))

(event EventTick
  (params (DeltaSeconds :type Float%20%28single-precision%29))
  (bind _asderek_bp (Utilities|Casting|CastToderek_bp (Game|GetPlayerCharacter 0)))
  (bind _asgravity_tool (Utilities|Casting|CastTogravity_tool (Variables|/Script/Engine.ChildActorComponent|GetChildActor (Variables|/Game/derek/derek_bp.derek_bp_C|GetTool _asderek_bp))))
  (if (Variables|/Game/assets/gravity_tool/gravity_tool.gravity_tool_C|GetHolding _asgravity_tool)
    (Utilities|IsValid (Variables|Default|GetCurrent%20Widget) :!label _label
      (:Is%20Valid
        (Rendering|SetVisibility (Variables|Default|GetCurrent%20Widget) false false)))
    (else
      (bind (_outhit _returnvalue) (Collision|LineTraceForObjects (Transformation|GetWorldLocation (Variables|/Game/derek/derek_bp.derek_bp_C|GetCasting%20Point _asderek_bp)) (+ (Transformation|GetWorldLocation (Variables|/Game/derek/derek_bp.derek_bp_C|GetCasting%20Point _asderek_bp)) (* (Math|Vector|GetForwardVector (Variables|/Game/derek/derek_bp.derek_bp_C|GetCasting%20Point _asderek_bp)) (Variables|/Game/assets/gravity_tool/gravity_tool.gravity_tool_C|GetGrabbing%20Distance _asgravity_tool))) (Variables|/Game/assets/gravity_tool/gravity_tool.gravity_tool_C|GetObject%20Types _asgravity_tool) false 0 "None"))
      (if _returnvalue
        (bind _asmoveable_bp (Utilities|Casting|CastToMoveable_BP (.hitactor _outhit))
          (:then
            (Variables|Default|SetHovered%20Object _asmoveable_bp)
            (Variables|Default|SetCurrent%20Widget (Variables|Moveable_BP_C|GetHover%20Widget _asmoveable_bp))
            (bind _ashover_widget (Utilities|Casting|CastToHover_Widget (UserInterface|GetUserWidgetObject (Variables|Moveable_BP_C|GetHover%20Widget _asmoveable_bp))))
            (Variables|/Game/assets/Hover_Widget.Hover_Widget_C|SetContent _ashover_widget (Utilities|Text|FormatText "{name} : {kg}KG" (Variables|Moveable_BP_C|GetUser%20Friendly%20Name _asmoveable_bp) (Variables|Moveable_BP_C|GetWeight _asmoveable_bp)))
            (Rendering|SetVisibility (Variables|Default|GetCurrent%20Widget) true false)
            (bind _asderek_bp_2 (Utilities|Casting|CastToderek_bp (Game|GetPlayerCharacter 0)))
            (Transformation|SetWorldTransform (Variables|Default|GetCurrent%20Widget) (Math|Transform|MakeTransform (+ (.Origin (Collision|GetActorBounds (Variables|Default|GetHovered%20Object) true)) (Math|Vector|MakeVector 0.0 0.0 (.z (.BoxExtent (Collision|GetActorBounds (Variables|Default|GetHovered%20Object) true))))) (Math|Rotator|FindLookatRotation (Transformation|GetWorldLocation (Variables|Default|GetCurrent%20Widget)) (Transformation|GetWorldLocation (Variables|/Game/derek/derek_bp.derek_bp_C|GetCasting%20Point _asderek_bp_2))) (Math|Vector|MakeVector 1.0 (Math|Float|Min(Float) (* (/ 1.0 (Math|Conversions|ToFloat(Integer) (Utilities|String|Len (Utilities|String|ToString(Text) (Utilities|Text|FormatText "{name} : {kg}KG" (Variables|Moveable_BP_C|GetUser%20Friendly%20Name _asmoveable_bp) (Variables|Moveable_BP_C|GetWeight _asmoveable_bp)))))) 8.0) 1.0) (Math|Float|Min(Float) (* (/ 1.0 (Math|Conversions|ToFloat(Integer) (Utilities|String|Len (Utilities|String|ToString(Text) (Utilities|Text|FormatText "{name} : {kg}KG" (Variables|Moveable_BP_C|GetUser%20Friendly%20Name _asmoveable_bp) (Variables|Moveable_BP_C|GetWeight _asmoveable_bp)))))) 8.0) 1.0))) false false))
          (:CastFailed
            (goto _label)))
        (else
          (goto _label))))))

(fn ConstructionScript)