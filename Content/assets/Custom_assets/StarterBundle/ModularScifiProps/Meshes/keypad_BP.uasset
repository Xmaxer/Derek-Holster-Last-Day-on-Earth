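; Keypad puzzle Blueprint that builds a code from key hits and checks it against a correct code.
; On BeginPlay it binds to the player derek_bp's key hit and hover dispatchers.
; Key object names act as input: digits append up to the code length, "delete" clears, and "enter" broadcasts the result, locking input on success.
; Hovering shows the bracketed key name through the Derek_UI widget.
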(event Custom|Key%20hit%20event
  (params (Key :type Primitive%20Component%20Object%20Reference))
  (bind _returnvalue (Utilities|GetObjectName Key))
  (bind _correct_code (Variables|Default|GetCorrect%20Code))
  (if (not (Variables|Default|GetCompleted))
    (Development|PrintString _returnvalue)
    (if (Utilities|Enum|Equal(Enum) _returnvalue "enter")
      (Default|CallKeyEnteredDispatcher (and (Utilities|Enum|Equal(Enum) _correct_code (stale _output_get)) (== (Utilities|String|Len (stale _output_get)) (Utilities|String|Len _correct_code))))
      (Variables|Default|SetCompleted (and (Utilities|Enum|Equal(Enum) _correct_code (stale _output_get)) (== (Utilities|String|Len (stale _output_get)) (Utilities|String|Len _correct_code))))
      (elif (Utilities|Enum|Equal(Enum) _returnvalue "delete")
        (Variables|Default|SetCode "")
        (elif (not (> (Utilities|String|Len (Utilities|String|Append (Variables|Default|GetCode) _returnvalue)) (Utilities|String|Len (Variables|Default|GetCorrect%20Code))))
          (bind _output_get (Variables|Default|SetCode (Utilities|String|Append (Variables|Default|GetCode) _returnvalue))))))))

(event Custom|Hovering%20event
  (params (Key :type Primitive%20Component%20Object%20Reference))
  (bind _foundwidgets (Widget|GetAllWidgetsOfClass "/Game/UI/Derek_UI.Derek_UI_C" true))
  (Default|ShowKey _foundwidgets (Utilities|Text|FormatText "[{key}]" (Utilities|Text|ToText(String) (Utilities|GetObjectName Key)))))

(event EventBeginPlay
  (bind _asderek_bp (Utilities|Casting|CastToderek_bp (Game|GetPlayerCharacter 0)))
  (EventDispatchers|BindEventtoKeyHitDispatcher _asderek_bp (delegate Custom|Key%20hit%20event))
  (EventDispatchers|BindEventtoKeyHoveredDispatcher _asderek_bp (delegate Custom|Hovering%20event)))

(fn ConstructionScript)