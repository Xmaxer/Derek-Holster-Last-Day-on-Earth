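; Elevator Blueprint that slides two doors open and closed.
; A DoorControl timeline drives the relative locations of the left and right doors, using the negated offset for the right so they move symmetrically apart.
; Open plays the timeline and, when TimerBased is set, reverses it after an OpenForSeconds delay, while Close reverses it directly.
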(event Custom|Open%20Door
  (bind _open_close_door (Timeline|Door%20Control Play)
    (:Update
      (Transformation|SetRelativeLocation (Variables|Default|Getelevator_door_left) _open_close_door false false)
      (Transformation|SetRelativeLocation (Variables|Default|Getelevator_door_right) (Math|Vector|NegateVector _open_close_door) false false))))

(event EventClose
  (bind _open_close_door (Timeline|Door%20Control Reverse)
    (:Update
      (Transformation|SetRelativeLocation (Variables|Default|Getelevator_door_left) _open_close_door false false)
      (Transformation|SetRelativeLocation (Variables|Default|Getelevator_door_right) (Math|Vector|NegateVector _open_close_door) false false))))

(event EventOpen
  (CallFunction|OpenDoor)
  (if (Variables|Default|GetTimer%20Based)
    (Utilities|FlowControl|Delay (Variables|Default|GetOpen%20For%20%28Seconds%29))
    (bind _open_close_door (Timeline|Door%20Control Reverse)
      (:Update
        (Transformation|SetRelativeLocation (Variables|Default|Getelevator_door_left) _open_close_door false false)
        (Transformation|SetRelativeLocation (Variables|Default|Getelevator_door_right) (Math|Vector|NegateVector _open_close_door) false false)))))

(fn ConstructionScript)