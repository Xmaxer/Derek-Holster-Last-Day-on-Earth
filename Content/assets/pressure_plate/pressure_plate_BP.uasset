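; Pressure plate Blueprint that opens linked Openable_BP actors when the total weight of Moveable_BP objects on it is within a min/max range.
; Area overlaps add and subtract weight: entering in range opens the Actionables, exceeding the maximum plays an error sound without closing them.
; Leaving closes them if the total is out of range, but never opens them.
; The Press timeline lowers the plate mesh by weight relative to the minimum, capped.
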(event OnComponentBeginOverlap(area)
  (params (OverlappedComponent :type Primitive%20Component%20Object%20Reference) (OtherActor :type Actor%20Object%20Reference) (OtherComp :type Primitive%20Component%20Object%20Reference) (OtherBodyIndex :type Integer) (bFromSweep :type Boolean) (SweepResult :type Hit%20Result%20Structure%20%28by%20ref%29))
  (bind _asmoveable_bp (Utilities|Casting|CastToMoveable_BP OtherActor))
  (bind _output_get (Variables|Default|SetTotal%20Weight (+ (Variables|/Game/assets/Moveable_BP.Moveable_BP_C|GetWeight _asmoveable_bp) (Variables|Default|GetTotal%20Weight))))
  (if (<= _output_get (Variables|Default|GetMax%20Weight))
    (if (>= _output_get (Variables|Default|GetMin%20Weight))
      (for _array_element (Variables|Default|GetActionables)
        (bind _asopenable_bp (Utilities|Casting|CastToOpenable_BP _array_element))
        (Default|Open _asopenable_bp)
        (bind _trigger (Timeline|Press PlayFromStart)
          (:Update
            (Transformation|SetRelativeLocation (Variables|Default|Getpressure_plate_pressure_plate_2) (Math|Vector|MakeVector 0.0 0.0 (Math|Float|Lerp (.z (Variables|/Script/Engine.SceneComponent|GetRelativeLocation (Variables|Default|Getpressure_plate_pressure_plate_2))) (* (Math|Float|Min(Float) (* (/ (Variables|Default|GetTotal%20Weight) (Variables|Default|GetMin%20Weight)) 8.0) 8.0) -1.0) _trigger)) false false)))))
    (else
      (Audio|PlaySoundatLocation "/Game/assets/pressure_plate/Pressure_Plate_Error.Pressure_Plate_Error" (Transformation|GetWorldLocation (Variables|Default|Getpressure_plate_platform)) "0, 0, 0" 1.0 1.0 0.0 0 0 0)
      (Timeline|Press PlayFromStart))))

(event OnComponentEndOverlap(area)
  (params (OverlappedComponent :type Primitive%20Component%20Object%20Reference) (OtherActor :type Actor%20Object%20Reference) (OtherComp :type Primitive%20Component%20Object%20Reference) (OtherBodyIndex :type Integer))
  (bind _asmoveable_bp (Utilities|Casting|CastToMoveable_BP OtherActor))
  (bind _output_get (Variables|Default|SetTotal%20Weight (- (Variables|Default|GetTotal%20Weight) (Variables|/Game/assets/Moveable_BP.Moveable_BP_C|GetWeight _asmoveable_bp))))
  (if (not (and (>= _output_get (Variables|Default|GetMin%20Weight)) (<= _output_get (Variables|Default|GetMax%20Weight))))
    (for _array_element (Variables|Default|GetActionables)
      (bind _asopenable_bp (Utilities|Casting|CastToOpenable_BP _array_element))
      (Default|Close _asopenable_bp)
      (bind _trigger (Timeline|Press PlayFromStart)
        (:Update
          (Transformation|SetRelativeLocation (Variables|Default|Getpressure_plate_pressure_plate_2) (Math|Vector|MakeVector 0.0 0.0 (Math|Float|Lerp (.z (Variables|/Script/Engine.SceneComponent|GetRelativeLocation (Variables|Default|Getpressure_plate_pressure_plate_2))) (* (Math|Float|Min(Float) (* (/ (Variables|Default|GetTotal%20Weight) (Variables|Default|GetMin%20Weight)) 8.0) 8.0) -1.0) _trigger)) false false))))))

(fn ConstructionScript)