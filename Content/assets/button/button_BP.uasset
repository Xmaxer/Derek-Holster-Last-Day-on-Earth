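; Button Blueprint that opens linked doors and animates its own press when triggered.
; DoAction loops over the Doors array, calls Open on each Openable_BP, and plays the TriggerButton timeline.
; After the timeline length, it calls UndoAction, which reverses the timeline to move the button mesh back via its relative location.
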(event EventDoAction
  (for _array_element (Variables|Default|GetDoors)
    (bind _asopenable_bp (Utilities|Casting|CastToOpenable_BP _array_element))
    (Default|Open _asopenable_bp)
    (bind _open_close_door (Timeline|Trigger%20Button Play)
      (:Update
        (Transformation|SetRelativeLocation (Variables|Default|Getbutton_button_2) _open_close_door false false))))
  (Utilities|FlowControl|Delay (Components|Timeline|GetTimelineLength (Variables|Default|GetTrigger%20Button)))
  (CallFunction|UndoAction))

(event EventUndoAction
  (bind _open_close_door (Timeline|Trigger%20Button Reverse)
    (:Update
      (Transformation|SetRelativeLocation (Variables|Default|Getbutton_button_2) _open_close_door false false))))

(fn ConstructionScript)